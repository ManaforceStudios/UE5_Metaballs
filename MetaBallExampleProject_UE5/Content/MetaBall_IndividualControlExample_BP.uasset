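; Metaball example Blueprint that drives individual balls in a metaball container from the positions of its scene components.
; When UseSceneObjectsAsTransforms is on, Tick feeds the relative location of eleven scene components to SetBallTransform by index.
; Each location has its axes reordered for the container's misaligned axes, is scaled into normalized bounding-box units, and is magnitude-clamped, as out-of-range values can crash the engine.
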(event EventBeginPlay)

(event Collision|EventActorBeginOverlap
  (params (OtherActor :type Actor%20Object%20Reference)))

(event EventTick
  (params (DeltaSeconds :type Float%20%28single-precision%29))
  (if (Variables|Default|GetUseSceneObjectsAsTransforms)
    (for (_array_element _array_index) (Utilities|Array|MakeArray (Variables|Default|GetScene) (Variables|Default|GetScene1) (Variables|Default|GetScene2) (Variables|Default|GetScene3) (Variables|Default|GetScene4) (Variables|Default|GetScene5) (Variables|Default|GetScene6) (Variables|Default|GetScene7) (Variables|Default|GetScene8) (Variables|Default|GetScene9) (Variables|Default|GetScene10))
      (Class|Metaballs|SetBallTransform _array_index (Math|Vector|ClampVectorSize (/ (Math|Vector|MakeVector (.Y (Math|Vector|BreakVector (Variables|/Script/Engine.SceneComponent|GetRelativeLocation _array_element))) (.Z (Math|Vector|BreakVector (Variables|/Script/Engine.SceneComponent|GetRelativeLocation _array_element))) (.X (Math|Vector|BreakVector (Variables|/Script/Engine.SceneComponent|GetRelativeLocation _array_element)))) 1e+02) -1.0 1.0)))))

(fn ConstructionScript)